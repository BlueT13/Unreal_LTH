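; Player character Blueprint that handles movement, look, jump and attack through Enhanced Input, adding IMC_MyPlayer on BeginPlay.
; Movement follows the actor's rotation, and look input drives controller yaw and pitch.
; Move and attack inputs set an AnimationKey state (Move, Attack, or Idle on completion).
; Disconnected nodes that write AnimationChangeKey directly on ABP_PlayerAnimation remain in the graph but never run.
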(event Input|EnhancedActionEvents|EnhancedInputActionIA_Attack
  (params (ActionValue :type Boolean) (ElapsedSeconds :type Float%20%28double-precision%29) (TriggeredSeconds :type Float%20%28double-precision%29) (InputAction :type Input%20Action%20Object%20Reference :default "/Game/TH/Input/IA_Attack.IA_Attack"))
  (:Started
    (Variables|Default|SetAnimationKey "Attack"))
  (:Completed
    (Variables|Default|SetAnimationKey "Idle")))

(event Input|EnhancedActionEvents|EnhancedInputActionIA_MyMovement
  (params (ActionValue :type Vector%202D%20Structure) (ElapsedSeconds :type Float%20%28double-precision%29) (TriggeredSeconds :type Float%20%28double-precision%29) (InputAction :type Input%20Action%20Object%20Reference :default "/Game/TH/Input/IA_MyMovement.IA_MyMovement"))
  (bind _returnvalue (Transformation|GetActorRotation))
  (:Triggered
    (Pawn|Input|AddMovementInput (Math|Vector|GetRightVector (Math|Rotator|MakeRotator (.roll _returnvalue) 0.0 (.yaw _returnvalue))) (.x ActionValue) false)
    (Pawn|Input|AddMovementInput (Math|Vector|GetForwardVector (Math|Rotator|MakeRotator 0.0 0.0 (.yaw (Transformation|GetActorRotation)))) (.y ActionValue) false)
    (Variables|Default|SetAnimationKey "Move"))
  (:Completed
    (Variables|Default|SetAnimationKey "Idle")))

(event Input|EnhancedActionEvents|EnhancedInputActionIA_MyLookAround
  (params (ActionValue :type Vector%202D%20Structure) (ElapsedSeconds :type Float%20%28double-precision%29) (TriggeredSeconds :type Float%20%28double-precision%29) (InputAction :type Input%20Action%20Object%20Reference :default "/Game/TH/Input/IA_MyLookAround.IA_MyLookAround"))
  (Pawn|Input|AddControllerYawInput (.x ActionValue))
  (Pawn|Input|AddControllerPitchInput (.y ActionValue)))

(event Input|EnhancedActionEvents|EnhancedInputActionIA_Jump
  (params (ActionValue :type Boolean) (ElapsedSeconds :type Float%20%28double-precision%29) (TriggeredSeconds :type Float%20%28double-precision%29) (InputAction :type Input%20Action%20Object%20Reference :default "/Game/TH/Input/IA_Jump.IA_Jump"))
  (Character|Jump))

(event EventBeginPlay
  (Input|AddMappingContext (PlayerController|LocalPlayerSubsystems|GetEnhancedInputLocalPlayerSubsystem (Game|GetPlayerController 0)) "/Game/TH/Input/IMC_MyPlayer.IMC_MyPlayer" 0 "(bIgnoreAllPressedKeysUntilRelease=True,bForceImmediately=False,bNotifyUserSettings=False)"))

(fn ConstructionScript)